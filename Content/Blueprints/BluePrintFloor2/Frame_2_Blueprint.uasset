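; Interactable gallery frame on the second floor that shows a caption about the 2009 Keyboard Cat meme.
; On Interact, it passes the caption to the player's FirstPersonHUD through DrawTextToScreen, waits ten seconds, then clears the text and turns drawing off.
; The caption is hardcoded in the event graph and the construction script is empty.
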(event EventInteract
  (bind _returnvalue (Game|GetPlayerController 0))
  (bind _returnvalue_2 (HUD|GetHUD _returnvalue))
  (Variables|Default|Settext "Keyboard Cat, 2009  
After performance artist Charlie Schmidt uploaded a video of his cat pretending 
 to play a keyboard on Youtube, another Youtube user created a mashup of  
Keyboard Cat with himself falling down. After posting that video, everyone  
started creating their own mashup. ")
  (bind _asfirst_person_hud (Utilities|Casting|CastToFirstPersonHUD _returnvalue_2))
  (Default|DrawTexttoScreen _asfirst_person_hud true (Variables|Default|Gettext))
  (Utilities|FlowControl|Delay 1e+01)
  (Variables|Default|Settext "")
  (bind _asfirst_person_hud_2 (Utilities|Casting|CastToFirstPersonHUD _returnvalue_2))
  (Default|DrawTexttoScreen _asfirst_person_hud_2 false (Variables|Default|Gettext)))

(fn ConstructionScript)