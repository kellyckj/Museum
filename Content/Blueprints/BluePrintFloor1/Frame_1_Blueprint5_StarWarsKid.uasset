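; Interactable frame Blueprint for a Floor 1 exhibit about the 2001 Star Wars Kid viral video.
; On Interact, it casts the player's HUD to FirstPersonHUD and draws a hardcoded description of the video and its cyberbullying impact on screen.
; After a ten-second delay, it clears the text and tells the HUD to stop drawing it.
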(event EventInteract
  (bind _returnvalue (Game|GetPlayerController 0))
  (bind _returnvalue_2 (HUD|GetHUD _returnvalue))
  (Variables|Default|Settex "Star Wars Kid, 2001 (Viral Video) 
A canadian student unintentionally filmed himself in a basement pretending to 
 be Darth Maul, and a couple of students found the clip and uploaded it on 
 Kazaa. The video became viral and the student became a victim of bullying, 
 contributing to one of the first cases of cyberbullying. ")
  (bind _asfirst_person_hud (Utilities|Casting|CastToFirstPersonHUD _returnvalue_2))
  (Default|DrawTexttoScreen _asfirst_person_hud true (Variables|Default|Gettex))
  (Utilities|FlowControl|Delay 1e+01)
  (Variables|Default|Settex "")
  (bind _asfirst_person_hud_2 (Utilities|Casting|CastToFirstPersonHUD _returnvalue_2))
  (Default|DrawTexttoScreen _asfirst_person_hud_2 false (Variables|Default|Gettex)))

(fn ConstructionScript
  (|CallParentFunction))