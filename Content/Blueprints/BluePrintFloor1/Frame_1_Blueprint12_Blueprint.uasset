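; Interactable picture frame Blueprint for the first floor that presents an info caption about the "Pancake Bunny" meme from 2001.
; On Interact, it casts the player's HUD to FirstPersonHUD and calls DrawTextToScreen with the hardcoded description.
; After a fixed delay, it clears the text and turns the on-screen drawing off.
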(event EventInteract
  (bind _returnvalue (Game|GetPlayerController 0))
  (bind _returnvalue_2 (HUD|GetHUD _returnvalue))
  (Variables|Default|Settex "Pancake Bunny, 2001 (Animal)  
This meme became popular by sending people a picture of the pancake bunny 
 alongside a caption saying “I have no idea what you’re talking about, so here’s 
 a bunny with a pancake on its head.” It gained traction after Hironori  
Akutagawa posted pictures of her bunny on her website. A user also posted it  
on a DVD talk forum, gaining traffic.  ")
  (bind _asfirst_person_hud (Utilities|Casting|CastToFirstPersonHUD _returnvalue_2))
  (Default|DrawTexttoScreen _asfirst_person_hud true (Variables|Default|Gettex))
  (Utilities|FlowControl|Delay 1e+01)
  (Variables|Default|Settex "")
  (bind _asfirst_person_hud_2 (Utilities|Casting|CastToFirstPersonHUD _returnvalue_2))
  (Default|DrawTexttoScreen _asfirst_person_hud_2 false (Variables|Default|Gettex)))

(fn ConstructionScript
  (|CallParentFunction))