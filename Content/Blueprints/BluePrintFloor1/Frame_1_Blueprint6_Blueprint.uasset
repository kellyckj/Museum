(event EventInteract
  (bind _returnvalue (Game|GetPlayerController 0))
  (bind _returnvalue_2 (HUD|GetHUD _returnvalue))
  (Variables|Default|Settex "All Your Base Are Belong to Us, 1998 (Pop Culture Reference) 
This became one of the first response and image-macro memes after a gif of 
 the opening sequence to the game Zero Wing was posted on a site Zany  
Video Game Quotes. It became widely spread in 2001 when overclock.org  
posted a voice over the quote. ")
  (bind _asfirst_person_hud (Utilities|Casting|CastToFirstPersonHUD _returnvalue_2))
  (Default|DrawTexttoScreen _asfirst_person_hud true (Variables|Default|Gettex))
  (Utilities|FlowControl|Delay 1e+01)
  (Variables|Default|Settex "")
  (bind _asfirst_person_hud_2 (Utilities|Casting|CastToFirstPersonHUD _returnvalue_2))
  (Default|DrawTexttoScreen _asfirst_person_hud_2 false (Variables|Default|Gettex)))

(fn ConstructionScript
  (|CallParentFunction))