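; Interactable exhibit Blueprint for a framed Baby Cha-Cha-Cha piece that shows the player a caption about the 1996 viral dancing baby video.
; On Interact it casts the first player's HUD to FirstPersonHUD and draws the hardcoded text on screen.
; After a ten-second delay it clears the text and tells the HUD to stop drawing it.
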(event EventInteract
  (bind _returnvalue (Game|GetPlayerController 0))
  (bind _returnvalue_2 (HUD|GetHUD _returnvalue))
  (Variables|Default|Settex "Baby Cha-Cha-Cha, 1996 (Viral Video) 
The dancing baby was created to showcase new CGI software by Kinetix  
Character Studio. When it appeared on the hit show Ally Mcbeal, it became  
one of the first viral phenomena.  
")
  (bind _asfirst_person_hud (Utilities|Casting|CastToFirstPersonHUD _returnvalue_2))
  (Default|DrawTexttoScreen _asfirst_person_hud true (Variables|Default|Gettex))
  (Utilities|FlowControl|Delay 1e+01)
  (Variables|Default|Settex "")
  (bind _asfirst_person_hud_2 (Utilities|Casting|CastToFirstPersonHUD _returnvalue_2))
  (Default|DrawTexttoScreen _asfirst_person_hud_2 false (Variables|Default|Gettex)))

(fn ConstructionScript
  (|CallParentFunction))