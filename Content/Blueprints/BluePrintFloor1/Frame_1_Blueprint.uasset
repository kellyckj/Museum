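; Frame 1 exhibit Blueprint that shows a museum-style blurb about the 1997 "Mr. T Ate My Balls" meme when the player interacts with it.
; The Interact event casts the player controller's HUD to FirstPersonHUD and passes the caption to DrawTextToScreen.
; After a ten-second delay, it calls the same function with empty text and drawing turned off to clear the screen.
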(event EventInteract
  (bind _returnvalue (Game|GetPlayerController 0))
  (bind _returnvalue_2 (HUD|GetHUD _returnvalue))
  (Variables|Default|Settext "Mr.T Ate My Balls, 1997  
“Mr. T Ate My Balls” brought together still-image and text, being one of the first  
internet memes. The meme’s creator, Nehal Patel, was a student at the  
University of Illinois, Urbana-Champaign at the time.")
  (bind _asfirst_person_hud (Utilities|Casting|CastToFirstPersonHUD _returnvalue_2))
  (Default|DrawTexttoScreen _asfirst_person_hud true (Variables|Default|Gettext))
  (Utilities|FlowControl|Delay 1e+01)
  (Variables|Default|Settext "")
  (bind _asfirst_person_hud_2 (Utilities|Casting|CastToFirstPersonHUD _returnvalue_2))
  (Default|DrawTexttoScreen _asfirst_person_hud_2 false (Variables|Default|Gettext)))

(fn ConstructionScript)