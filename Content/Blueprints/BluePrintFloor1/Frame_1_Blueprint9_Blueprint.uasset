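; Interactable museum-style frame for floor 1 that shows a short history of the ROFLcopter meme when the player interacts with it.
; Interact stores the blurb in a text variable and passes it to the FirstPersonHUD's DrawTextToScreen.
; After a ten-second delay it clears the text and tells the HUD to stop drawing.
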(event EventInteract
  (bind _returnvalue (Game|GetPlayerController 0))
  (bind _returnvalue_2 (HUD|GetHUD _returnvalue))
  (Variables|Default|Settex "ROFLcopter, 2000-2001 (Slang) 
The term was first allegedly coined on a Warcraft III forum for trolling purposes. 
 It became one of the earliest ASCII art. A website, roflcopter.com, was  
registered with the gif of the helicopter, spreading the ROFLcopter usage. ")
  (bind _asfirst_person_hud (Utilities|Casting|CastToFirstPersonHUD _returnvalue_2))
  (Default|DrawTexttoScreen _asfirst_person_hud true (Variables|Default|Gettex))
  (Utilities|FlowControl|Delay 1e+01)
  (Variables|Default|Settex "")
  (bind _asfirst_person_hud_2 (Utilities|Casting|CastToFirstPersonHUD _returnvalue_2))
  (Default|DrawTexttoScreen _asfirst_person_hud_2 false (Variables|Default|Gettex)))

(fn ConstructionScript
  (|CallParentFunction))