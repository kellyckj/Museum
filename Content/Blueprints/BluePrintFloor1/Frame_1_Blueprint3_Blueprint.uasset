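; Interactable frame Blueprint that shows an informational caption about the 1999 Hamster Dance website.
; On Interact, it stores the hard-coded text and passes it to the player's FirstPersonHUD through DrawTextToScreen.
; After a ten-second delay, it clears the text and switches the HUD drawing off.
; The construction script only calls its parent.
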(event EventInteract
  (bind _returnvalue (Game|GetPlayerController 0))
  (bind _returnvalue_2 (HUD|GetHUD _returnvalue))
  (Variables|Default|Settex "Hamster Dance, 1999 
The Hamster Dance was one of the earliest single-purpose websites. It was  
created by Canadian art student Deidre LeCarte after competing with her sister 
 to see who can generate the most web traffic. The site had over 17 million  
visits in 1999.  
")
  (bind _asfirst_person_hud (Utilities|Casting|CastToFirstPersonHUD _returnvalue_2))
  (Default|DrawTexttoScreen _asfirst_person_hud true (Variables|Default|Gettex))
  (Utilities|FlowControl|Delay 1e+01)
  (Variables|Default|Settex "")
  (bind _asfirst_person_hud_2 (Utilities|Casting|CastToFirstPersonHUD _returnvalue_2))
  (Default|DrawTexttoScreen _asfirst_person_hud_2 false (Variables|Default|Gettex)))

(fn ConstructionScript
  (|CallParentFunction))