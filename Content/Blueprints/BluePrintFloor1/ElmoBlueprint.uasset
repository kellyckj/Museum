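; ElmoBlueprint is an interactable exhibit that shows an informational caption about the "Bert is Evil" parody website.
; On Interact, it casts the first player's HUD to FirstPersonHUD and passes the hardcoded text to DrawTextToScreen.
; After a timed Delay, it clears the text and turns drawing off through the same HUD call.
; The construction script only calls its parent.
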(event EventInteract
  (bind _returnvalue (Game|GetPlayerController 0))
  (bind _returnvalue_2 (HUD|GetHUD _returnvalue))
  (Variables|Default|Settex "Bert Is Evil, 1998 
Bert is Evil is a parody website that was started by Dino Ignacio. The  
website distorted Bert into political figures and events such as the  
assassination of JFK and the Oklahoma City bombing. Later it was used  
in a pro Osama Bin Laden protest rally.   
")
  (bind _asfirst_person_hud (Utilities|Casting|CastToFirstPersonHUD _returnvalue_2))
  (Default|DrawTexttoScreen _asfirst_person_hud true (Variables|Default|Gettex))
  (Utilities|FlowControl|Delay 1e+01)
  (Variables|Default|Settex "")
  (bind _asfirst_person_hud_2 (Utilities|Casting|CastToFirstPersonHUD _returnvalue_2))
  (Default|DrawTexttoScreen _asfirst_person_hud_2 false (Variables|Default|Gettex)))

(fn ConstructionScript
  (|CallParentFunction))