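; Interactable floor 1 frame exhibit that shows a short history blurb about the 1996 Saltine Challenge.
; On Interact, it sends the hard-coded text to the player's FirstPersonHUD through DrawTextToScreen.
; After a ten-second delay it clears the text and turns drawing off.
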(event EventInteract
  (bind _returnvalue (Game|GetPlayerController 0))
  (bind _returnvalue_2 (HUD|GetHUD _returnvalue))
  (Variables|Default|Settex "Saltine Challenge, 1996 
Though the Saltine Challenge became a popular game on Youtube in 2012, it 
t was first reported on the news in the early 1990’s. In 1996, Los Angeles  
Times reported that football player Peyton Manning attempted the challenge. 
")
  (bind _asfirst_person_hud (Utilities|Casting|CastToFirstPersonHUD _returnvalue_2))
  (Default|DrawTexttoScreen _asfirst_person_hud true (Variables|Default|Gettex))
  (Utilities|FlowControl|Delay 1e+01)
  (Variables|Default|Settex "")
  (bind _asfirst_person_hud_2 (Utilities|Casting|CastToFirstPersonHUD _returnvalue_2))
  (Default|DrawTexttoScreen _asfirst_person_hud_2 false (Variables|Default|Gettex)))

(fn ConstructionScript
  (|CallParentFunction))