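; Interactable frame Blueprint on floor 1 that shows an informational caption about the "It's a Trap!" meme from 2000.
; On Interact, it casts the player's HUD to FirstPersonHUD and passes the hard-coded text to DrawTextToScreen.
; After a ten-second delay, it clears the text and turns the on-screen drawing off.
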(event EventInteract
  (bind _returnvalue (Game|GetPlayerController 0))
  (bind _returnvalue_2 (HUD|GetHUD _returnvalue))
  (Variables|Default|Settex "It's a Trap!, 2000 (Catchphrase) 
This reaction image became popular after Something Awful administrator  
OMGWTFBBQ created and uploaded a picture from a scene from Star Wars 
: Return of the Jedi. It was used often to warn someone of deception. ")
  (bind _asfirst_person_hud (Utilities|Casting|CastToFirstPersonHUD _returnvalue_2))
  (Default|DrawTexttoScreen _asfirst_person_hud true (Variables|Default|Gettex))
  (Utilities|FlowControl|Delay 1e+01)
  (Variables|Default|Settex "")
  (bind _asfirst_person_hud_2 (Utilities|Casting|CastToFirstPersonHUD _returnvalue_2))
  (Default|DrawTexttoScreen _asfirst_person_hud_2 false (Variables|Default|Gettex)))

(fn ConstructionScript
  (|CallParentFunction))