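; Button actor that works as an overlap trigger, signalling when something enters or leaves it.
; Begin and end overlap set the Inttrigger flag and share one branch, which calls Buttontrue on entry and Buttonfalse on exit.
; Both paths toggle the TextRender's visibility, so the text flips on every overlap event with no filter on the overlapping actor.
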(event Collision|EventActorBeginOverlap
  (params (OtherActor :type Actor%20Object%20Reference))
  (Variables|Default|Setinttrigger true)
  (if (Variables|Default|Getinttrigger)
    (Rendering|ToggleVisibility (Variables|Default|GetTextRender) false)
    (Default|CallButtontrue)
    (else
      (Rendering|ToggleVisibility (Variables|Default|GetTextRender) false)
      (Default|CallButtonfalse))))

(event Collision|EventActorEndOverlap
  (params (OtherActor :type Actor%20Object%20Reference))
  (Variables|Default|Setinttrigger false)
  (if (Variables|Default|Getinttrigger)
    (Rendering|ToggleVisibility (Variables|Default|GetTextRender) false)
    (Default|CallButtontrue)
    (else
      (Rendering|ToggleVisibility (Variables|Default|GetTextRender) false)
      (Default|CallButtonfalse))))

(fn ConstructionScript)